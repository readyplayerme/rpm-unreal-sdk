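; Half-body avatar preview actor for the Ready Player Me avatar creator, rendered through a scene capture showing only itself.
; Events swap the skeletal mesh, rotate it, and reset the view on gender change.
; The capture camera eases or zooms between NearPin and FarPin components.
; New meshes are rescaled using a feminine preset or, when their height ratio to the initial mesh exceeds a threshold, that ratio clamped.
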(event EventBeginPlay
  (Rendering|SceneCapture|ShowOnlyActorComponents (Variables|Default|GetSceneCaptureComponent2D) self false)
  (Variables|Default|SetInitialHalfBodyHeight (.z (.boxextent (StaticMesh|GetBounds (Class|RpmAvatarCreatorFunctionLibrary|GetSkeletalMeshfromComponent (Variables|Default|GetAvatarMesh)))))))

(event EventUpdateAvatar
  (params (SkeletalMesh :type Skeletal%20Mesh%20Object%20Reference))
  (bind _avatarmesh (Variables|Default|GetAvatarMesh))
  (Class|SkinnedMeshComponent|SetSkeletalMesh _avatarmesh SkeletalMesh false)
  (CallFunction|SetMeshScale _avatarmesh (Variables|Default|GetInitialHalfBodyHeight)))

(event EventUpdateGender
  (params (Gender :type EAvatarGender%20Enum :default "Undefined"))
  (Variables|Default|SetGender Gender)
  (Transformation|SetRelativeRotation (Variables|Default|GetAvatarMesh) "0, 0, 0" false false)
  (Transformation|SetRelativeTransform (Variables|Default|GetSceneCaptureComponent2D) (Transformation|GetRelativeTransform (Variables|Default|GetNearPin)) false false))

(event EventRotateAvatar
  (params (Delta :type Float%20%28single-precision%29))
  (Transformation|AddRelativeRotation (Variables|Default|GetAvatarMesh) (Math|Rotator|MakeRotator 0.0 0.0 (* Delta (Variables|Default|GetActorRotationSpeed))) false false))

(event EventZoomCamera
  (params (Delta :type Float%20%28single-precision%29))
  (Transformation|SetRelativeTransform (Variables|Default|GetSceneCaptureComponent2D) (CallFunction|GetZoomTransform Delta) false false))

(event EventMoveCamera
  (params (ToFace :type Boolean))
  (bind _destination (CallFunction|GetDestinationTransform ToFace))
  (Components|MoveComponentTo (Variables|Default|GetSceneCaptureComponent2D) (.location _destination) (.rotation _destination) true false 0.3 false))

(fn ConstructionScript)

(fn GetZoomTransform
  (params (Delta :type Float%20%28single-precision%29))
  (bind _scenecapturecomponent2d (Variables|Default|GetSceneCaptureComponent2D))
  (bind _returnvalue (Transformation|GetRelativeTransform _scenecapturecomponent2d))
  (Utilities|FlowControl|Sequence
    (:then_0
      ;[1 1 1] Comment
      (if (>= Delta 0.0)
        (LocalVariables|SetDestinationZoomLocation (Variables|/Script/Engine.SceneComponent|GetRelativeLocation (Variables|Default|GetNearPin)))
        (else
          (LocalVariables|SetDestinationZoomLocation (Variables|/Script/Engine.SceneComponent|GetRelativeLocation (Variables|Default|GetFarPin))))))
    (:then_1
      ;[1 1 1] Comment
      (return (Math|Transform|MakeTransform (- (.location _returnvalue) (* (Math|Vector|Normalize (- (.location _returnvalue) (LocalVariables|GetDestinationZoomLocation))) (Math|Float|Min(Float) (Math|Float|Absolute(Float) (* Delta (Variables|Default|GetActorZoomSpeed))) (Math|Vector|Distance(Vector) (.location _returnvalue) (LocalVariables|GetDestinationZoomLocation))))) (.rotation _returnvalue) "1,1,1")))))

(fn GetDestinationTransform
  (params (ToFace :type Boolean))
  (if ToFace
    (return (Transformation|GetRelativeTransform (Variables|Default|GetNearPin)))
    (else
      (return (Transformation|GetRelativeTransform (Variables|Default|GetFarPin))))))

(fn SetMeshScale
  (params (MeshComponent :type Skeletal%20Mesh%20Component%20Object%20Reference) (InitialHeight :type Float%20%28single-precision%29))
  (bind _returnvalue (Class|RpmAvatarCreatorFunctionLibrary|GetSkeletalMeshfromComponent MeshComponent))
  (bind _meshscalethreshold (Variables|Default|GetMeshScaleThreshold))
  (bind _returnvalue_2 (- 1.0 _meshscalethreshold))
  (bind _returnvalue_3 (StaticMesh|GetBounds _returnvalue))
  (bind _returnvalue_4 (+ 1.0 _meshscalethreshold))
  (bind _returnvalue_5 (/ InitialHeight (.z (.boxextent _returnvalue_3))))
  (Utilities|FlowControl|Sequence
    (:then_0
      ;[1 1 1] Set Female Mesh Scale
      (if (Utilities|Enum|Equal(Enum) (Variables|Default|GetGender) "Feminine")
        (LocalVariables|SetScale 1.05)))
    (:then_1
      ;[1 1 1] Clamp Scale
      (if (not (Math|Float|InRange(Float) _returnvalue_5 _returnvalue_2 _returnvalue_4))
        (LocalVariables|SetScale (Math|Float|Clamp(Float) _returnvalue_5 _returnvalue_2 _returnvalue_4))))
    (:then_2
      ;[1 1 1] Set Final Scale
      (Transformation|SetRelativeScale3D MeshComponent (Math|Conversions|ToVector(Float) (LocalVariables|GetScale))))))

(fn GetBackgroundMaterial
  (return "/ReadyPlayerMe/ReadyPlayerMe/AvatarCreator/Materials/M_RPM_EditorBG.M_RPM_EditorBG"))

(fn GetRenderMaterial
  (return "/ReadyPlayerMe/ReadyPlayerMe/AvatarCreator/Materials/M_RPM_PreviewRenderMaterial.M_RPM_PreviewRenderMaterial"))

(fn GetRenderTargetSize
  ;[1 1 1] Return Render Target Dimentions
  (return "(X=1536.000000,Y=1024.000000)"))